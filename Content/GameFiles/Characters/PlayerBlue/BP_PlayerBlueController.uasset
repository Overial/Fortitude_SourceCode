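; Player controller for the PlayerBlue character that carries out its ranged weapon attack.
; On BeginPlay it caches player 0's pawn as a BP_PlayerBlueCharacter.
; The OnAttackRanged event spawns a scaled-down bullet at the weapon mesh's Muzzle socket transform, along with a small explosion emitter and a firing sound at that location.
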(event `self.ReceiveBeginPlay`
  (bind _asbp_player_blue_character (cast `/Game/GameFiles/Characters/PlayerBlue/BP_PlayerBlueCharacter` (`GameplayStatics.GetPlayerCharacter` 0)))
  (set `self.PlayerBlueCharacter` _asbp_player_blue_character))

(event `self.OnAttackRanged`
  (bind (_returnvalue_location _returnvalue_rotation) (`KismetMathLibrary.BreakTransform` (`SceneComponent.GetSocketTransform` (`FortitudePlayerCharacter.WeaponMesh` (`self.PlayerBlueCharacter`)) "Muzzle" "RTS_World")))
  (`|SpawnActorFromClass` "/Game/GameFiles/Blueprints/Bullet/BP_PlayerBlue_Bullet.BP_PlayerBlue_Bullet_C" (`KismetMathLibrary.MakeTransform` _returnvalue_location _returnvalue_rotation (0.7 0.7 0.7)) "Undefined" "OverrideRootScale" null null)
  (`GameplayStatics.SpawnEmitterAtLocation` "/Game/StarterContent/Particles/P_Explosion.P_Explosion" _returnvalue_location (struct) (0.3 0.3 0.3))
  (`GameplayStatics.PlaySoundAtLocation` "/Game/FirstPerson/Audio/A_PlayerBlue_Fire_Cue.A_PlayerBlue_Fire_Cue" _returnvalue_location (struct) 1.0 1.0 0.0 null null null))

(fn `UserConstructionScript`
  (`parent.UserConstructionScript`))