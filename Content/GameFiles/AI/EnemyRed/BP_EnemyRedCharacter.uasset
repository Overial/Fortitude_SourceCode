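; BP_EnemyRedCharacter is the red enemy character Blueprint, defining how it reacts to death.
; When its HealthComponent fires OnDie, a DoOnce-guarded branch plays the death montage on the mesh.
; A second sequence branch briefly slows global time and lowers audio pitch, then restores both after a delay, giving a slow-motion death effect.
; The construction script only calls its parent.
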(event `self.HealthComponent.OnDie`
  (`|ExecutionSequence`
    (:`then_0`
      (`/Engine/EditorBlueprintResources/StandardMacros.DoOnce` false
        (:`Completed`
          (`|PlayMontage` (`self.Mesh`) "/Game/AnimStarterPack/AM_EnemyRed_Death.AM_EnemyRed_Death"))))
    (:`then_1`
      (`GameplayStatics.SetGlobalTimeDilation` 0.3)
      (`GameplayStatics.SetGlobalPitchModulation` 0.3)
      (`KismetSystemLibrary.Delay` 0.5)
      (`GameplayStatics.SetGlobalTimeDilation` 1.0)
      (`GameplayStatics.SetGlobalPitchModulation` 1.0))))

(fn `UserConstructionScript`
  (`parent.UserConstructionScript`))