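; Blue player bullet Blueprint that damages enemies on hit.
; It handles OnBulletTargetHit, acting only on valid actors tagged Enemy.
; A hit applies BaseDamage credited to the first player controller and player character, plays a click sound at the bullet's location, then destroys the bullet.
; The construction script only calls its parent.
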(event `self.OnBulletTargetHit`
  (params (OtherActor :type "Actor Object Reference"))
  (`/Engine/EditorBlueprintResources/StandardMacros.IsValid` OtherActor
    (:`Is Valid`
      (if (`self.ActorHasTag` OtherActor "Enemy")
        (`GameplayStatics.ApplyDamage` OtherActor (`self.BaseDamage`) (`GameplayStatics.GetPlayerController` 0) (`GameplayStatics.GetPlayerCharacter` 0))
        (`GameplayStatics.PlaySoundAtLocation` "/Engine/VREditor/Sounds/UI/Click_on_Button.Click_on_Button" (`self.K2_GetActorLocation`) (struct) 1.0 1.0 0.0 null null null)
        (`self.K2_DestroyActor`)))))

(fn `UserConstructionScript`
  (`parent.UserConstructionScript`))