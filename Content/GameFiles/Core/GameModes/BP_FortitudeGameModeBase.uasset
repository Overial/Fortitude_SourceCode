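; Base game mode for Fortitude that sets up input and starts the game's music when play begins.
; BeginPlay sets the first player controller to game-only input.
; Outside development mode, it has BP_FortitudeGameInstance initialize and play music, but only if CombatMusic is not yet valid, so music already held by the game instance is not recreated.
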(event `self.ReceiveBeginPlay`
  (`|ExecutionSequence`
    (:`then_0`
      (`WidgetBlueprintLibrary.SetInputMode_GameOnly` (`GameplayStatics.GetPlayerController` 0)))
    (:`then_1`
      (if (not (`self.IsInDevelopmentMode?`))
        (bind _asbp_fortitude_game_instance (cast `/Game/GameFiles/Core/GameInstances/BP_FortitudeGameInstance` (`GameplayStatics.GetGameInstance`)))
        (`/Game/GameFiles/Core/GameInstances/BP_FortitudeGameInstance.CombatMusic` _asbp_fortitude_game_instance
          (:`then`)
          (:`else`
            (`/Game/GameFiles/Core/GameInstances/BP_FortitudeGameInstance.FnInitMusic` _asbp_fortitude_game_instance)
            (`/Game/GameFiles/Core/GameInstances/BP_FortitudeGameInstance.FnPlayMusic` _asbp_fortitude_game_instance)))))))

(fn `UserConstructionScript`)