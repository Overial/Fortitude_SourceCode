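; BP_FortitudeGameInstance is a game instance that holds the Player and Enemy scores, round restarts and combat music.
; A score update event increments the winner's tally, and a new round event reloads Level_01 after a short delay.
; Music is created once as a 2D sound set to persist across level transitions, then started by a separate play function that flags it as playing.
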(event `self.OnUpdateScore`
  (params (Winner :type "ERoundWinner Enum" :default "Player"))
  (switch `ERoundWinner` Winner
    (:`Player`
      (`/Engine/EditorBlueprintResources/StandardMacros.IncrementInt` (`self.PlayerScore`)))
    (:`Enemy`
      (`/Engine/EditorBlueprintResources/StandardMacros.IncrementInt` (`self.EnemyScore`)))))

(event `self.OnNewRound`
  (`KismetSystemLibrary.Delay` 3.0)
  (`GameplayStatics.OpenLevel` "Level_01"))

(fn `FnInitMusic`
  (bind _returnvalue (`GameplayStatics.CreateSound2D` "/Game/GameFiles/Sounds/Music/A_CP2077_RebelPath_Cue.A_CP2077_RebelPath_Cue" 1.0 1.0 0.0 null true))
  (set `self.CombatMusic` _returnvalue))

(fn `FnPlayMusic`
  (bind _combatmusic (`self.CombatMusic`)
    (:`then`
      (`AudioComponent.Play` _combatmusic 0.0)
      (set `self.IsMusicPlaying?` true))
    (:`else`)))